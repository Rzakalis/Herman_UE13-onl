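; Base player character Blueprint that handles walking, looking, sprinting and crouching through Enhanced Input actions.
; Movement follows control yaw only, while look input drives controller yaw and inverted-sign pitch.
; Sprint and crouch are hold-to-use: sprint swaps max walk speed, and crouch calls Crouch/UnCrouch while updating an IsCrouching flag.
; On BeginPlay it hides the mesh's head bone.
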(event Input|EnhancedActionEvents|EnhancedInputActionIA_UE13Loock
  (params (ActionValue :type Vector%202D%20Structure) (ElapsedSeconds :type Float%20%28double-precision%29) (TriggeredSeconds :type Float%20%28double-precision%29) (InputAction :type Input%20Action%20Object%20Reference :default "/Game/UE13/Blueprints/Character/Input/IA_UE13Loock.IA_UE13Loock"))
  (Pawn|Input|AddControllerYawInput (.x ActionValue))
  (Pawn|Input|AddControllerPitchInput (* (.y ActionValue) -1.0)))

(event Input|EnhancedActionEvents|EnhancedInputActionIA_UE13Move
  (params (ActionValue :type Vector%202D%20Structure) (ElapsedSeconds :type Float%20%28double-precision%29) (TriggeredSeconds :type Float%20%28double-precision%29) (InputAction :type Input%20Action%20Object%20Reference :default "/Game/UE13/Blueprints/Character/Input/IA_UE13Move.IA_UE13Move"))
  (bind _returnvalue (Pawn|GetControlRotation :!class /Script/Engine.Pawn))
  (bind _yaw (Math|Rotator|BreakRotator _returnvalue))
  (bind _returnvalue_2 (Math|Rotator|MakeRotator 0.0 0.0 _yaw))
  (Pawn|Input|AddMovementInput (Math|Vector|GetForwardVector _returnvalue_2) (.y ActionValue) false)
  (Pawn|Input|AddMovementInput (Math|Vector|GetRightVector _returnvalue_2) (.x ActionValue) false))

(event Input|EnhancedActionEvents|EnhancedInputActionIA_UE13Sprint
  (params (ActionValue :type Boolean) (ElapsedSeconds :type Float%20%28double-precision%29) (TriggeredSeconds :type Float%20%28double-precision%29) (InputAction :type Input%20Action%20Object%20Reference :default "/Game/UE13/Blueprints/Character/Input/IA_UE13Sprint.IA_UE13Sprint"))
  (bind _charactermovement (Variables|Character|GetCharacterMovement))
  (:Started
    (Variables|/Script/Engine.CharacterMovementComponent|SetMaxWalkSpeed _charactermovement 3.5e+02))
  (:Completed
    (Variables|/Script/Engine.CharacterMovementComponent|SetMaxWalkSpeed _charactermovement 2e+02)))

(event Input|EnhancedActionEvents|EnhancedInputActionIA_UE13Crouch
  (params (ActionValue :type Boolean) (ElapsedSeconds :type Float%20%28double-precision%29) (TriggeredSeconds :type Float%20%28double-precision%29) (InputAction :type Input%20Action%20Object%20Reference :default "/Game/UE13/Blueprints/Character/Input/IA_UE13Crouch.IA_UE13Crouch"))
  (:Started
    (Character|Crouch)
    (Variables|Default|SetIsCrouching true))
  (:Completed
    (Character|UnCrouch)
    (Variables|Default|SetIsCrouching false)))

(event EventBeginPlay
  (Components|SkinnedMesh|HideBonebyName (Variables|Character|GetMesh) "head" "PBO_None"))

(fn ConstructionScript)