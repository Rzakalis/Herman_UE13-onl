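; BP_Trigger is a trigger box actor that steps through staged visual changes each time the player overlaps it.
; The first overlap hides two lights and the 3D text, then restores the lights and shows the mannequin after a delay.
; The next three apply DT_TriggerVisual rows: light colors, then also relative offsets for the mannequin, and finally other components too.
; Count, row data and current state print for debugging.
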(event OnComponentBeginOverlap(Box)
  (params (OverlappedComponent :type Primitive%20Component%20Object%20Reference) (OtherActor :type Actor%20Object%20Reference) (OtherComp :type Primitive%20Component%20Object%20Reference) (OtherBodyIndex :type Integer) (bFromSweep :type Boolean) (SweepResult :type Hit%20Result%20Structure%20%28by%20ref%29))
  (if (== OtherActor (Game|GetPlayerCharacter 0))
    (bind _output_get (Variables|Default|SetCount (+ 1 (Variables|Default|GetCount))))
    (Development|PrintString (Utilities|String|ToString(Integer) _output_get))
    (switch int _output_get
      (:1
        (Rendering|SetVisibility (Variables|Default|GetPointLight1) false false)
        (Rendering|SetVisibility (Variables|Default|GetPointLight2) false false)
        (Rendering|SetVisibility (Variables|Default|GetText3D) false false)
        (Utilities|FlowControl|Delay 2.0)
        (Rendering|SetVisibility (Variables|Default|GetPointLight1) true false)
        (Rendering|SetVisibility (Variables|Default|GetPointLight2) true false)
        (Rendering|SetVisibility (Variables|Default|GetSKM_Manny_Simple) true false))
      (:2
        (bind _out_row_light_color (CallFunction|GetVisualfromDataTable "1"))
        (Rendering|Components|Light|SetLightColor (Variables|Default|GetPointLight1) _out_row_light_color true)
        (Variables|Default|SetCurrentStateName "1")
        (CallFunction|PrintDatafromTable (Variables|Default|GetCurrentStateName)))
      (:3
        (bind (_outdata _out_row_name _out_row_light_color_2 _out_row_mesh_off_set) (CallFunction|GetVisualfromDataTable "2"))
        (Rendering|Components|Light|SetLightColor (Variables|Default|GetPointLight2) _out_row_light_color_2 true)
        (Transformation|SetRelativeLocation (Variables|Default|GetSKM_Manny_Simple) _out_row_mesh_off_set false true)
        (Variables|Default|SetCurrentStateName "2")
        (CallFunction|PrintDatafromTable (Variables|Default|GetCurrentStateName)))
      (:4
        (bind (_outdata_2 _out_row_name_2 _out_row_light_color_3 _out_row_mesh_off_set_2) (CallFunction|GetVisualfromDataTable "3"))
        (Rendering|Components|Light|SetLightColor (Variables|Default|GetPointLight1) _out_row_light_color_3 true)
        (Rendering|Components|Light|SetLightColor (Variables|Default|GetPointLight2) _out_row_light_color_3 true)
        (Transformation|SetRelativeLocation (Variables|Default|GetSKM_Manny_Simple) _out_row_mesh_off_set_2 false true)
        (Transformation|SetRelativeLocation (Variables|Default|GetSM_Cube) _out_row_mesh_off_set_2 false true)
        (Transformation|SetRelativeLocation (Variables|Default|GetSM_Cube1) _out_row_mesh_off_set_2 false true)
        (Transformation|SetRelativeLocation (Variables|Default|GetPointLight) _out_row_mesh_off_set_2 false true)
        (Transformation|SetRelativeLocation (Variables|Default|GetText3D) _out_row_mesh_off_set_2 false true)
        (Variables|Default|SetCurrentStateName "3")
        (CallFunction|PrintDatafromTable (Variables|Default|GetCurrentStateName))))))

(fn ConstructionScript)

(fn GetVisualfromDataTable
  (params (RowName :type Name))
  (bind _returnvalue (Utilities|GetDataTableRow "/Game/UE13/Blueprints/DT_TriggerVisual.DT_TriggerVisual" RowName)
    (:then
      (Development|PrintString (Utilities|String|ToString(Name) (.name _returnvalue))))
    (:RowNotFound
      _))
  (return "" (.name _returnvalue) (.lightcolor _returnvalue) (.meshoffset _returnvalue)))

(fn PrintDatafromTable
  (params (RowNameInput :type Name))
  (bind _returnvalue (Utilities|GetDataTableRow "/Game/UE13/Blueprints/DT_TriggerVisual.DT_TriggerVisual" RowNameInput)
    (:then
      (Development|PrintString (Utilities|String|ToString(Text) (Utilities|Text|FormatText "State: {Name} | Color: {Color} | Offset: {Offset}" (.Name (Utilities|Struct|BreakST_TriggerVisualData _returnvalue)) (Utilities|String|ToString(Integer) (.LightColor (Utilities|Struct|BreakST_TriggerVisualData _returnvalue))) (Utilities|String|ToString(Vector) (.MeshOffSet (Utilities|Struct|BreakST_TriggerVisualData _returnvalue)))))))))