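; BP_Elevator is an elevator actor that travels between its starting position and a fixed point above it.
; On BeginPlay it records both endpoints.
; Each time the player character begins overlapping its Box, a FlipFlop alternates between playing and reversing MoveTimeline.
; The timeline's Alpha lerps the actor between the endpoints with a swept SetActorLocation.
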(event OnComponentBeginOverlap(Box)
  (params (OverlappedComponent :type Primitive%20Component%20Object%20Reference) (OtherActor :type Actor%20Object%20Reference) (OtherComp :type Primitive%20Component%20Object%20Reference) (OtherBodyIndex :type Integer) (bFromSweep :type Boolean) (SweepResult :type Hit%20Result%20Structure%20%28by%20ref%29))
  (if (== OtherActor (Game|GetPlayerCharacter 0))
    (Utilities|FlowControl|FlipFlop
      (:A
        (bind _alpha (Timeline|MoveTimeline Play)
          (:Update
            (Transformation|SetActorLocation (Math|Vector|Lerp(Vector) (Variables|Default|GetStartLocation) (Variables|Default|GetEndLocation) _alpha) true false))))
      (:B
        (Timeline|MoveTimeline Reverse)))))

(event EventBeginPlay
  (bind _output_get (Variables|Default|SetStartLocation (Transformation|GetActorLocation)))
  (Variables|Default|SetEndLocation (+ _output_get "0.000000,0.000000,450.000000")))

(fn ConstructionScript)